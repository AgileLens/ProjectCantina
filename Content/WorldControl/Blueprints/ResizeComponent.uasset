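; Actor component that lets two hands resize and reposition its owning actor, adding a Grab Component on BeginPlay if the owner lacks one.
; BeginResize stores both hands, their starting distance and the actor's scale, then starts resizing after a short delay.
; Until EndResize, Tick multiplies that scale by the hand-distance ratio and teleports the actor to the hands' midpoint.
; Haptic feedback and debug prints are present but disconnected.
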(event `self.ReceiveBeginPlay`
  ;[0 0.6449 1] If Actor doesn't also have Grab Component, add it
  (bind _output_get (set `self.OwningActor` (`self.GetOwner`)))
  (`/Engine/EditorBlueprintResources/StandardMacros.IsValid` (`Actor.GetComponentByClass` _output_get "/Game/VRTemplate/Blueprints/GrabComponent.GrabComponent_C")
    (:`Is Not Valid`
      (`|AddComponentByClass` :`self` (`self.OwningActor`) :`Class` "/Game/VRTemplate/Blueprints/GrabComponent.GrabComponent_C"))))

(event `/Game/WorldControl/Blueprints/ResizeActorInterface.BeginResize`
  (params (FirstHand :type "SceneComponent Object Reference") (SecondHand :type "SceneComponent Object Reference"))
  (`self.SetComponentTickEnabled` true)
  (set `self.FirstHand` FirstHand)
  (set `self.SecondHand` SecondHand)
  (bind _distance (`/Game/WorldControl/Blueprints/BPFL_GetDistance.GetDistance` (`self.FirstHand`) (`self.SecondHand`)))
  (set `self.InitialDistance` _distance)
  (bind _output_get (set `self.InitialScale` (`Actor.GetActorScale3D` (`self.GetOwner`))))
  (`KismetSystemLibrary.Delay` 0.1)
  (set `self.bIsResizing` true))

(event `self.ReceiveTick`
  (params (DeltaSeconds :type "Float (single-precision)"))
  (bind _returnvalue (`self.GetOwner`))
  (if (`self.bIsResizing`)
    (bind _distance (`/Game/WorldControl/Blueprints/BPFL_GetDistance.GetDistance` (`self.FirstHand`) (`self.SecondHand`)))
    (bind _output_get (set `self.CurrentScale` (* (`self.InitialScale`) (/ _distance (`self.InitialDistance`)))))
    (`Actor.SetActorScale3D` _returnvalue _output_get)
    (`Actor.K2_SetActorLocation` _returnvalue (/ (+ (`self.K2_GetComponentLocation` (`self.FirstHand`)) (`self.K2_GetComponentLocation` (`self.SecondHand`))) 2) false true)))

(event `/Game/WorldControl/Blueprints/ResizeActorInterface.EndResize`
  (set `self.bIsResizing` false)
  (`self.SetComponentTickEnabled` false))